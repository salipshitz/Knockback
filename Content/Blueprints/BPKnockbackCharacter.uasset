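; First-person player character with a charge-up gun that knocks its shooter backwards, with movement, look and jump disabled once dead.
; Releasing fire or touch launches the character opposite the camera and spawns a knockback projectile, both scaled by hold time with a one-second floor.
; Die extends the parent, hiding the HUD and swapping to the death camera and third-person mesh.
; Releasing Jump also calls Die.
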(event Input|ActionEvents|InputActionJump
  (params (Key :type Key%20Structure :default "None"))
  (:Pressed
    (if (not (Variables|Default|GetDead))
      (Character|Jump)))
  (:Released
    (Character|StopJumping)
    (CallFunction|Die)))

(event Input|ActionEvents|InputActionFire
  (params (Key :type Key%20Structure :default "None"))
  (bind _returnvalue (Transformation|GetActorLocation))
  (bind _dead (Variables|Default|GetDead))
  (bind _firstpersoncamera (Variables|MyCharacter|GetFirstPersonCamera))
  (bind _returnvalue_2 (Transformation|GetWorldRotation _firstpersoncamera))
  (:Pressed
    (if (not _dead)
      (Variables|Default|SetChargeTime (Utilities|Time|GetGameTimeinSeconds))))
  (:Released
    (if (not _dead)
      (Animation|Montage|MontagePlay (Components|SkeletalMesh|GetAnimInstance (Variables|MyCharacter|GetMesh2P)) "/Game/FirstPerson/Animations/FirstPersonFire_Montage.FirstPersonFire_Montage" 1.0 "MontageLength" 0.0 true)
      (Character|LaunchCharacter (* (Math|Vector|GetForwardVector _returnvalue_2) (* (* (Math|Float|SelectFloat 1.0 (- (Utilities|Time|GetGameTimeinSeconds) (Variables|Default|GetChargeTime)) (< (- (Utilities|Time|GetGameTimeinSeconds) (Variables|Default|GetChargeTime)) 1.0)) 1e+03) -1.0)) false false)
      (bind _returnvalue_3 (Game|SpawnActorfromClass "/Game/Blueprints/BPKnockbackProjectile.BPKnockbackProjectile_C" (Math|Transform|MakeTransform (+ (Transformation|GetWorldLocation (Variables|Default|GetSphere)) (Math|Vector|RotateVector (Variables|Default|GetGunOffset) _returnvalue_2)) _returnvalue_2) "AlwaysSpawn" 0 0)) ; Spawn projectile
      (Variables|/Game/Blueprints/BPKnockbackProjectile.BPKnockbackProjectile_C|SetForce _returnvalue_3 (* (Math|Float|SelectFloat 1.0 (- (Utilities|Time|GetGameTimeinSeconds) (Variables|Default|GetChargeTime)) (< (- (Utilities|Time|GetGameTimeinSeconds) (Variables|Default|GetChargeTime)) 1.0)) 1e+03))
      (Audio|PlaySoundatLocation "/Game/StarterContent/Audio/Explosion02.Explosion02" _returnvalue "0, 0, 0" 1.0 1.0 0.0 0 0 0)
      (Class|AISenseHearing|ReportNoiseEvent _returnvalue 1.0 self 0.0 "Noise"))))

(event Input|AxisEvents|InputAxisTurn
  (params (AxisValue :type Float%20%28single-precision%29))
  (if (not (Variables|Default|GetDead))
    (Pawn|Input|AddControllerYawInput AxisValue)))

(event Input|AxisEvents|InputAxisLookUp
  (params (AxisValue :type Float%20%28single-precision%29))
  (if (not (Variables|Default|GetDead))
    (Pawn|Input|AddControllerPitchInput AxisValue)))

(event Input|AxisEvents|InputAxisMoveForward
  (params (AxisValue :type Float%20%28single-precision%29))
  (if (not (Variables|Default|GetDead))
    (Pawn|Input|AddMovementInput (Transformation|GetActorForwardVector) AxisValue false)))

(event Input|AxisEvents|InputAxisMoveRight
  (params (AxisValue :type Float%20%28single-precision%29))
  (if (not (Variables|Default|GetDead))
    (Pawn|Input|AddMovementInput (Transformation|GetActorRightVector) AxisValue false)))

(event Input|AxisEvents|InputAxisTurnRate
  (params (AxisValue :type Float%20%28single-precision%29))
  (if (not (Variables|Default|GetDead))
    (Pawn|Input|AddControllerYawInput (* AxisValue (Variables|Default|GetBaseTurnRate) (Utilities|Time|GetWorldDeltaSeconds)))))

(event Input|AxisEvents|InputAxisLookUpRate
  (params (AxisValue :type Float%20%28single-precision%29))
  (if (not (Variables|Default|GetDead))
    (Pawn|Input|AddControllerPitchInput (* AxisValue (Variables|Default|GetBaseLookUpRate) (Utilities|Time|GetWorldDeltaSeconds)))))

(event Input|TouchEvents|InputTouch
  (params (Location :type Vector) (FingerIndex :type ETouchIndex%20Enum))
  (bind _returnvalue (Transformation|GetActorLocation))
  (bind _dead (Variables|Default|GetDead))
  (bind _firstpersoncamera (Variables|MyCharacter|GetFirstPersonCamera))
  (bind _returnvalue_2 (Transformation|GetWorldRotation _firstpersoncamera))
  (:Pressed
    (if (not _dead)
      (Variables|Default|SetChargeTime (Utilities|Time|GetGameTimeinSeconds))))
  (:Released
    (if (not _dead)
      (Animation|Montage|MontagePlay (Components|SkeletalMesh|GetAnimInstance (Variables|MyCharacter|GetMesh2P)) "/Game/FirstPerson/Animations/FirstPersonFire_Montage.FirstPersonFire_Montage" 1.0 "MontageLength" 0.0 true)
      (Character|LaunchCharacter (* (Math|Vector|GetForwardVector _returnvalue_2) (* (* (Math|Float|SelectFloat 1.0 (- (Utilities|Time|GetGameTimeinSeconds) (Variables|Default|GetChargeTime)) (< (- (Utilities|Time|GetGameTimeinSeconds) (Variables|Default|GetChargeTime)) 1.0)) 1e+03) -1.0)) false false)
      (bind _returnvalue_3 (Game|SpawnActorfromClass "/Game/Blueprints/BPKnockbackProjectile.BPKnockbackProjectile_C" (Math|Transform|MakeTransform (+ (Transformation|GetWorldLocation (Variables|Default|GetSphere)) (Math|Vector|RotateVector (Variables|Default|GetGunOffset) _returnvalue_2)) _returnvalue_2) "AlwaysSpawn" 0 0)) ; Spawn projectile
      (Variables|/Game/Blueprints/BPKnockbackProjectile.BPKnockbackProjectile_C|SetForce _returnvalue_3 (* (Math|Float|SelectFloat 1.0 (- (Utilities|Time|GetGameTimeinSeconds) (Variables|Default|GetChargeTime)) (< (- (Utilities|Time|GetGameTimeinSeconds) (Variables|Default|GetChargeTime)) 1.0)) 1e+03))
      (Audio|PlaySoundatLocation "/Game/StarterContent/Audio/Explosion02.Explosion02" _returnvalue "0, 0, 0" 1.0 1.0 0.0 0 0 0)
      (Class|AISenseHearing|ReportNoiseEvent _returnvalue 1.0 self 0.0 "Noise"))))

(fn ConstructionScript
  (Transformation|AttachComponentToComponent (Variables|Default|GetFP_Gun) (Variables|MyCharacter|GetMesh2P) "GripPoint" "SnapToTarget" "SnapToTarget" "SnapToTarget" true))

(fn Die
  (|CallParentFunction)
  (Variables|/Script/Engine.HUD|SetbShowHUD (HUD|GetHUD (Game|GetPlayerController 0)) false)
  (Components|Activation|Activate (Variables|Default|GetDeathCamera) false)
  (Components|Activation|Deactivate (Variables|MyCharacter|GetFirstPersonCamera))
  (Class|PrimitiveComponent|SetOwnerNoSee (Variables|Character|GetMesh) false)
  (Class|PrimitiveComponent|SetOwnerNoSee (Variables|MyCharacter|GetMesh2P) true)
  (Class|PrimitiveComponent|SetOwnerNoSee (Variables|Default|GetFP_Gun) true))