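; BPKnockbackProjectile is a projectile that applies knockback to what it hits, scaled by Force.
; Its Hit event pushes physics-simulating components with an impulse along its velocity, or launches Characters in its direction of travel.
; Otherwise it calls BlowUp on a BPBarrel.
; It destroys itself after any of these or on hitting a StaticMeshActor, but survives other hits.
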(event Collision|EventHit
  (params (MyComp :type Primitive%20Component%20Object%20Reference) (Other :type Actor%20Object%20Reference) (OtherComp :type Primitive%20Component%20Object%20Reference) (bSelfMoved :type Boolean) (HitLocation :type Vector :default "0, 0, 0") (HitNormal :type Vector :default "0, 0, 0") (NormalImpulse :type Vector :default "0, 0, 0") (Hit :type Hit%20Result%20Structure%20%28by%20ref%29))
  (bind _returnvalue (Transformation|GetVelocity))
  (bind _force (Variables|Default|GetForce))
  (if (Physics|IsSimulatingPhysics OtherComp "None")
    (Physics|AddImpulseatLocation OtherComp (* _returnvalue (/ _force 1e+01)) (Transformation|GetActorLocation) "None")
    (else
      (bind _ascharacter (Utilities|Casting|CastToCharacter Other)
        (:then
          (Character|LaunchCharacter _ascharacter (* (Math|Vector|Normalize _returnvalue) _force) false false))
        (:CastFailed
          (bind _asbpbarrel (Utilities|Casting|CastToBPBarrel Other)
            (:then
              (Default|BlowUp _asbpbarrel))
            (:CastFailed
              (Utilities|Casting|CastToStaticMeshActor Other)))))))
  (Actor|DestroyActor))

(fn ConstructionScript)