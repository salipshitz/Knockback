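; GunnerCharacter is a gun-carrying character Blueprint that dies when it lands from a fall.
; Its construction script snaps FPGun onto the GripPoint socket of Mesh2P.
; Tick watches for falling, records the start time, and calls Die on landing without checking that time, so any fall is fatal.
; Die runs the parent implementation, then makes the controller unpossess the character.
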(event EventTick
  (params (DeltaSeconds :type Float%20%28single-precision%29))
  (if (AI|Components|NavMovement|IsFalling (Variables|Character|GetCharacterMovement))
    (if (not (Variables|Default|GetAlreadyFalling))
      (Variables|Default|SetAlreadyFalling true)
      (Variables|Default|SetInitialFallTime (Utilities|Time|GetTimeSeconds)))
    (elif (Variables|Default|GetAlreadyFalling)
      (Variables|Default|SetAlreadyFalling false)
      (CallFunction|Die))))

(fn ConstructionScript
  (Transformation|AttachComponentToComponent (Variables|Default|GetFP_Gun) (Variables|MyCharacter|GetMesh2P) "GripPoint" "SnapToTarget" "SnapToTarget" "SnapToTarget" true))

(fn Die
  (|CallParentFunction)
  (Pawn|UnPossess (Pawn|GetController)))